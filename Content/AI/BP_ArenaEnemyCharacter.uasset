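; Arena enemy character that shows its current AI state on a debug text component.
; Every Tick it casts its controller to BP_ArenaEnemyAIController and reads the BB_ArenaEnemy blackboard.
; InAttackRange, HasLOS and TargetActor validity are checked in priority order to set a colour-coded label: attacking, chasing, lost or patrolling.
; It calls UseBlackboard on every update to get the blackboard component.
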(event `self.ReceiveTick`
  (params (DeltaSeconds :type "Float (single-precision)"))
  (`self.UpdateDebugText`))

(fn `UpdateDebugText`
  (bind _debugtext (`self.DebugText`))
  (bind _asbp_arena_enemy_aicontroller (cast `/Game/AI/BP_ArenaEnemyAIController` (`self.GetController`)))
  (bind _blackboardcomponent (`AIController.UseBlackboard` _asbp_arena_enemy_aicontroller "/Game/AI/BB_ArenaEnemy.BB_ArenaEnemy"))
  (if (`BlackboardComponent.GetValueAsBool` _blackboardcomponent (`.SelectedKeyName` (break `BlackboardKeySelector` (make `BlackboardKeySelector` :`SelectedKeyName` "InAttackRange"))))
    (`TextRenderComponent.SetTextRenderColor` _debugtext (make `Color` 0 0 255))
    (`TextRenderComponent.K2_SetText` _debugtext "ATTACKING")
    (elif (`BlackboardComponent.GetValueAsBool` _blackboardcomponent (`.SelectedKeyName` (break `BlackboardKeySelector` (make `BlackboardKeySelector` :`SelectedKeyName` "HasLOS"))))
      (`TextRenderComponent.SetTextRenderColor` _debugtext (make `Color` 0 255 255))
      (`TextRenderComponent.K2_SetText` _debugtext "CHASING")
      (else
        (`/Engine/EditorBlueprintResources/StandardMacros.IsValid` (`BlackboardComponent.GetValueAsObject` _blackboardcomponent (`.SelectedKeyName` (break `BlackboardKeySelector` (make `BlackboardKeySelector` :`SelectedKeyName` "TargetActor"))))
          (:`Is Valid`
            (`TextRenderComponent.SetTextRenderColor` _debugtext (make `Color` 255))
            (`TextRenderComponent.K2_SetText` _debugtext "LOST"))
          (:`Is Not Valid`
            (`TextRenderComponent.SetTextRenderColor` _debugtext (make `Color` 0 255))
            (`TextRenderComponent.K2_SetText` _debugtext "PATROLLING")))))))

(fn `UserConstructionScript`)